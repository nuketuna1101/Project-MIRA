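; Marksman trooper character Blueprint for MIRA that adds the feedback played when the trooper dies.
; BeginPlay binds to OnDead, and a DoOnce-gated handler plays a death sound, then runs three custom effect events.
; Knockback launches the body along the damage causer's forward vector, CameraShake plays a world shake centred on the causer, and DeadStop drives global time dilation from a timeline for slow motion.
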(event `self.ReceiveBeginPlay`
  (add `MIRABaseCharacter.OnDead` (delegate `OnDeadMMTrooper`)))

(event `OnDeadMMTrooper`
  (params (DamageCauser :type "Actor Object Reference"))
  (`/Engine/EditorBlueprintResources/StandardMacros.DoOnce` false
    (:`Completed`
      (`GameplayStatics.PlaySoundAtLocation` "/Game/MIRA/Audio/SQ_SFX_MMTrooperDeath.SQ_SFX_MMTrooperDeath" (`self.K2_GetActorLocation`) (struct) 1.0 1.0 0.0 null null null null)
      (`self.Knockback` DamageCauser)
      (`self.CameraShake` (`self.K2_GetActorLocation` DamageCauser) true)
      (`self.DeadStop`))))

(event `Knockback`
  (params (Causer :type "Actor Object Reference"))
  ;[1 1 1] Custom Event: Knockback
  (`self.LaunchCharacter` (* (`self.GetActorForwardVector` Causer) 2000.0))
  (`self.SetActorEnableCollision` true))

(event `CameraShake`
  (params (Epicenter :type "Vector Structure") (IsHigher :type Boolean))
  ;[1 1 1] Custom Event: Camera Shake
  (if IsHigher
    (`GameplayStatics.PlayWorldCameraShake` null Epicenter 1000.0 2500.0)
    (else
      (`GameplayStatics.PlayWorldCameraShake` null Epicenter 1000.0 2500.0 1.0 true))))

(event `DeadStop`
  ;[1 1 1] Custom Efx: slow motion
  (bind (_direction `_새_트랙_0`) (`Timeline|타임라인` :!via `PlayFromStart`)
    (:`Update`
      (`GameplayStatics.SetGlobalTimeDilation` `_새_트랙_0`))))

(fn `UserConstructionScript`)